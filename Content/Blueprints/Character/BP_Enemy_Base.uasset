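; Base enemy character Blueprint that handles the visual side of spawning, turning toward a target and dissolving.
; On BeginPlay a timeline drives the mesh's uniform scale as a spawn effect.
; UpdateFacingTarget feeds a location into the MotionWarping "FacingTarget" warp target.
; Separate body and weapon timelines animate the "Dissolve" scalar on dynamic material instances passed in by the caller.
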(event `self.ReceiveBeginPlay`
  (bind (_direction _scaletrack) (`Timeline|SpawnTimeline`)
    (:`Update`
      (`SceneComponent.SetRelativeScale3D` (`self.Mesh`) (`KismetMathLibrary.MakeVector` _scaletrack _scaletrack _scaletrack)))))

(event `AuraCombatInterface.UpdateFacingTarget`
  (params (TargetLocation :type "Vector Structure (by ref)"))
  ; Updates the actor to face the target
  (`MotionWarpingComponent.AddOrUpdateWarpTargetFromLocation` (`self.MotionWarping`) "FacingTarget" TargetLocation))

(event `self.StartDissolveTimeline`
  (params (DynamicMaterialInstance :type "MaterialInstanceDynamic Object Reference"))
  ; Dissolve Effect - Mesh and Weapon
  (bind (_direction _dissolvetrack) (`Timeline|DissolveTimeline`)
    (:`Update`
      (`MaterialInstanceDynamic.SetScalarParameterValue` DynamicMaterialInstance "Dissolve" _dissolvetrack))))

(event `self.StartWeaponDissolveTimeline`
  (params (DynamicMaterialInstance :type "MaterialInstanceDynamic Object Reference"))
  ; Dissolve Effect - Mesh and Weapon
  (bind (_direction _weapondissolve) (`Timeline|WeaponDissolveTimeline`)
    (:`Update`
      (`MaterialInstanceDynamic.SetScalarParameterValue` DynamicMaterialInstance "Dissolve" _weapondissolve))))

(fn `UserConstructionScript`)