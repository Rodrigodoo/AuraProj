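; BP_AuraCharacter is the Aura character Blueprint, handling attack-style facing warps and fading of objects that block the camera's view of the character.
; UpdateFacingTarget feeds a location into Motion Warping as the FacingTarget warp target.
; Box overlap begin and end events, on the locally controlled instance only, call FadeObstacle, which sends fade-out or fade-in messages to actors implementing BI_FadeInterface.
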(event `AuraCombatInterface.UpdateFacingTarget`
  (params (TargetLocation :type "Vector Structure (by ref)"))
  (`MotionWarpingComponent.AddOrUpdateWarpTargetFromLocation` (`self.MotionWarping`) "FacingTarget" TargetLocation))

(event `self.Box.OnComponentBeginOverlap`
  (params (OverlappedComponent :type "PrimitiveComponent Object Reference") (OtherActor :type "Actor Object Reference") (OtherComp :type "PrimitiveComponent Object Reference") (OtherBodyIndex :type Integer) (bFromSweep :type Boolean) (SweepResult :type "HitResult Structure (by ref)"))
  ; If something is between the camera and the character, try to fade it out
  (if (`self.IsLocallyControlled`)
    (`self.FadeObstacle` OtherActor true)))

(event `self.Box.OnComponentEndOverlap`
  (params (OverlappedComponent :type "PrimitiveComponent Object Reference") (OtherActor :type "Actor Object Reference") (OtherComp :type "PrimitiveComponent Object Reference") (OtherBodyIndex :type Integer))
  ; When the object is no longer between the camera and the character, fade it back in
  (if (`self.IsLocallyControlled`)
    (`self.FadeObstacle` OtherActor)))

(fn `FadeObstacle`
  (params (Actor :type "Actor Object Reference") (FadeOut :type Boolean))
  (if (`KismetSystemLibrary.DoesImplementInterface` Actor "/Game/Blueprints/Actor/FadeActor/BI_FadeInterface.BI_FadeInterface_C")
    (if (`local.FadeOut`)
      (message `/Game/Blueprints/Actor/FadeActor/BI_FadeInterface.FadeOut` (`local.Actor`))
      (else
        (message `/Game/Blueprints/Actor/FadeActor/BI_FadeInterface.FadeIn` (`local.Actor`))))))

(fn `UserConstructionScript`)