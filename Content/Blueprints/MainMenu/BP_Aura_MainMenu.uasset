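; BP_Aura_MainMenu is a main menu Blueprint that makes its FireBall component bob up and down.
; BeginPlay caches the fireball's starting world location.
; Each Tick accumulates a Time value, reset to zero after a full 2π period, then sets the fireball's Z to the starting height plus a sine of Time scaled by Amplitude.
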(event `self.ReceiveBeginPlay`
  (set `self.FireBallInitialLocation` (`SceneComponent.K2_GetComponentLocation` (`self.FireBall`))))

(event `self.ReceiveTick`
  (params (DeltaSeconds :type "Float (single-precision)"))
  (`self.UpdateTime` DeltaSeconds)
  (`self.UpdateFireBallLocation`))

(fn `UpdateFireBallLocation`
  (bind (_fireballinitiallocation_x _fireballinitiallocation_y _fireballinitiallocation_z) (`KismetMathLibrary.BreakVector` (`self.FireBallInitialLocation`)))
  (`SceneComponent.K2_SetWorldLocation` (`self.FireBall`) (`KismetMathLibrary.MakeVector` _fireballinitiallocation_x _fireballinitiallocation_y (+ _fireballinitiallocation_z (* (`KismetMathLibrary.Sin` (`self.Time`)) (`self.Amplitude`)))) false false))

(fn `UpdateTime`
  (params (DeltaTime :type "Float (double-precision)"))
  (bind _output_get (set `self.Time` (+ DeltaTime (`self.Time`))))
  (if (> _output_get (`KismetMathLibrary.GetTAU`))
    ; Reset Time after hitting a full period (2Pi)
    (set `self.Time` 0.0)))

(fn `UserConstructionScript`)