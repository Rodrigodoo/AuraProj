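; Passive gameplay ability for Aura that listens for attribute gameplay events and turns them into changes on its owner.
; On activation it waits for any event under the Attributes tag, child tags included, and never ends itself.
; Each event's tag and magnitude become a SetByCaller value on an EventBasedEffectClass spec applied to self, so one effect class serves every attribute tag.
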(event `self.K2_ActivateAbility`
  (bind (_asynctaskproxy _payload) (`AbilityTask_WaitGameplayEvent.WaitGameplayEvent` (struct :`TagName` "Attributes") null false false)
    (:`EventReceived`
      (bind (_eventtag _instigator _target _optionalobject _optionalobject2 _contexthandle _instigatortags _targettags _eventmagnitude) (break `GameplayEventData` _payload))
      (`self.ApplyEventBased Effect` _eventtag _eventmagnitude))))

(fn `ApplyEventBased Effect`
  (params (EventTag :type "GameplayTag Structure") (Magnitude :type "Float (single-precision)"))
  (bind _returnvalue (`self.GetAbilitySystemComponentFromActorInfo`))
  (bind _returnvalue_2 (`AbilitySystemBlueprintLibrary.AssignTagSetByCallerMagnitude` (`AbilitySystemComponent.MakeOutgoingSpec` _returnvalue (`self.EventBasedEffectClass`) 1.0 (`AbilitySystemComponent.MakeEffectContext` _returnvalue)) EventTag Magnitude))
  (`AbilitySystemComponent.BP_ApplyGameplayEffectSpecToSelf` (`self.GetAbilitySystemComponentFromActorInfo`) _returnvalue_2))