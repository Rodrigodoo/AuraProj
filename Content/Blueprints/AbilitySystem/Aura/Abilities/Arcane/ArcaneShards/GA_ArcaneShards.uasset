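; Arcane Shards gameplay ability: shows a magic circle, waits for a confirming press, then erupts a series of shards around the targeted point.
; A spawned BP_PointCollection supplies randomly rotated ground points while the avatar plays a cast montage.
; The montage's gameplay event starts a looping timer that, per point, applies radial damage to non-friends and fires a gameplay cue.
; After the last shard or failed targeting, it cleans up and ends.
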(event `self.K2_ActivateAbility`
  (`|ExecutionSequence`
    (:`then_0`
      ; Show the magic circle
      (message `AuraPlayerInterface.ShowMagicCircle` (`self.GetAvatarActorFromActorInfo`) null))
    (:`then_1`
      ; Wait For Input press to call the ability
      (`AbilityTask_WaitInputPress.WaitInputPress` false
        (:`OnPress`
          (bind (_asynctaskproxy _datahandle) (`AuraTargetDataUnderMouse.CreateTargetDataUnderMouse`)
            (:`ValidData`
              (bind (_bblockinghit _binitialoverlap _time _distance _location _impactpoint) (`GameplayStatics.BreakHitResult` (`AbilitySystemBlueprintLibrary.GetHitResultFromTargetData` _datahandle)))
              (if _bblockinghit
                ; Get Ground Points
                (`self.CalculateGroundPoints` _impactpoint)
                ; Play Montage and Wait
                (message `AuraCombatInterface.UpdateFacingTarget` (`self.GetAvatarActorFromActorInfo`) _impactpoint)
                (`AbilityTask_PlayMontageAndWait.CreatePlayMontageAndWaitProxy` "None" (`self.Montage to Play`)
                  (:`then`
                    (`AbilityTask_WaitGameplayEvent.WaitGameplayEvent` (struct :`TagName` "Event.Montage.ArcaneShards") null true
                      (:`EventReceived`
                        ; Spawn Shards - Async
                        (bind _returnvalue (`KismetSystemLibrary.K2_SetTimerDelegate` (delegate `SpawnShard`) (`self.ShardSpawnDeltaTime`) true))
                        (set `self.ShardSpawnTimer` _returnvalue)
                        ;; Spawn the first shard Immediatly
                        (`self.SpawnShard`)
                        ;; Hide the Magic Circle
                        (message `AuraPlayerInterface.HideMagicCircle` (`self.GetAvatarActorFromActorInfo`))))))
                (else
                  (`KismetSystemLibrary.K2_ClearAndInvalidateTimerHandle` (`self.ShardSpawnTimer`) :!label _label)
                  (`KismetSystemLibrary.Delay` 0.2)
                  (bind _pointcollection (`self.PointCollection`)
                    (:`then`
                      (`Actor.K2_DestroyActor` _pointcollection)
                      (set `self.Count` 0)
                      (`KismetArrayLibrary.Array_Clear` (`self.GroundPoints`)))
                    (:`else`
                      _))
                  (`self.K2_EndAbilityLocally`))))
            (:`OnFailed`
              (goto _label))))))))

(event `SpawnShard`
  (bind (_output_location _output_rotation) (`KismetMathLibrary.BreakTransform` (`|GetArrayItem` (`self.GroundPoints`) (`self.Count`))))
  ; Spawn Shards - Async
  (if (< (`self.Count`) (`self.Num Points`))
    (`self.ApplyRadialDamageEffect` _output_location)
    (`self.K2_ExecuteGameplayCueWithParams` (struct :`TagName` "GameplayCue.ArcaneShards") (`AbilitySystemBlueprintLibrary.MakeGameplayCueParameters` 0.0 0.0 (struct) (struct) (struct) (struct) (struct) _output_location (`KismetMathLibrary.GetUpVector` _output_rotation)))
    (`/Engine/EditorBlueprintResources/StandardMacros.IncrementInt` (`self.Count`))
    (else
      (goto _label))))

(fn `ApplyRadialDamageEffect`
  (params (RadialDamageOrigin :type "Vector Structure"))
  (bind _returnvalue (`self.GetAvatarActorFromActorInfo`))
  (bind _outoverlappingactors (`AuraAbilitySystemLibrary.GetLivePlayerWithinRadius` _returnvalue (`|MakeArray` _returnvalue) (`self.RadialDamageOuterRadius`) (`local.RadialDamageOrigin`)))
  (for _array_element _outoverlappingactors
    (if (`AuraAbilitySystemLibrary.IsNotFriend` _array_element (`self.GetAvatarActorFromActorInfo`))
      (bind _structout (setmembers `AuraDamageEffectParams` :`StructRef` (`self.MakeDamageEffectParamsFromClassDefaults` _array_element) :`RadialDamageOrigin` (`local.RadialDamageOrigin`)))
      (`AuraAbilitySystemLibrary.ApplyDamageGameplayEffect` _structout))))

(fn `CalculateGroundPoints`
  (params (GroundPointOriginLocation :type "Vector Structure"))
  (bind _returnvalue (`|SpawnActorFromClass` "/Game/Blueprints/AbilitySystem/Aura/Abilities/Arcane/ArcaneShards/BP_PointCollection.BP_PointCollection_C" (`KismetMathLibrary.MakeTransform` GroundPointOriginLocation) "AlwaysSpawn" "MultiplyWithRoot" null null))
  (bind _output_get (set `self.PointCollection` _returnvalue))
  (set `self.GroundPoints` (`AuraPointCollection.GetGroundPoints` _output_get (`self.Num Points`) (`KismetMathLibrary.RandomFloatInRange` 0.0 360.0) 1500.0)))