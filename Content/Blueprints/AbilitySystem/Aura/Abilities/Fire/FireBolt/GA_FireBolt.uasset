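; Fire Bolt gameplay ability that casts homing projectiles at the target under the mouse.
; After checking cost and cooldown, it waits for mouse target data, commits, turns the avatar toward the hit and plays the cast montage.
; A montage gameplay event triggers the projectile spawn, with launch pitch scaled by socket-to-target distance up to a cap.
; The ability ends when the montage finishes, is interrupted or cancelled, or targeting fails.
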(event `self.K2_ActivateAbility`
  (bind _returnvalue (`BlueprintGameplayTagLibrary.MakeLiteralGameplayTag` (struct :`TagName` "Montage.Attack.Weapon")))
  ; Check the cooldown and spend the mana for this Abilitiy
  ; Note: Fails if still on cooldown or do not have enough mana
  (bind _returnvalue_2 (`self.CanCommitAbility`))
  (if _returnvalue_2
    (bind (_asynctaskproxy _datahandle) (`AuraTargetDataUnderMouse.CreateTargetDataUnderMouse`)
      (:`ValidData`
        (`self.K2_CommitAbility`)
        (bind (_bblockinghit _binitialoverlap _time _distance _location _impactpoint _normal _impactnormal _physmat _hitactor) (`GameplayStatics.BreakHitResult` (`AbilitySystemBlueprintLibrary.GetHitResultFromTargetData` _datahandle)))
        (set `self.ProjectileTargetLocation` _location)
        (set `self.TargetActor` _hitactor)
        ; When this Ability is activated, rotate the character towards the target, play the Fire Bolt montage and when the arm is full stretched emit a Gameplay Event to spawn the projectile
        (bind _asaura_combat_interface (cast `AuraCombatInterface` (`self.GetAvatarActorFromActorInfo`)))
        (`AuraCombatInterface.UpdateFacingTarget` _asaura_combat_interface (`self.ProjectileTargetLocation`))
        (`AbilityTask_PlayMontageAndWait.CreatePlayMontageAndWaitProxy` "None" "/Game/Assets/Characters/Aura/Animations/Abilities/AM_Cast_FireBolt.AM_Cast_FireBolt" 1.0 "None" false
          (:`then`
            (`AbilityTask_WaitGameplayEvent.WaitGameplayEvent` (struct :`TagName` "Event.Montage.FireBolt") null
              (:`EventReceived`
                (`self.SpawnProjectiles` (`self.ProjectileTargetLocation`) _returnvalue (`self.TargetActor`) true (`self.PitchOverrideCalculation` _returnvalue 800.0 45.0)))))
          (:`OnCompleted`
            (`self.K2_EndAbility` :!label _label))
          (:`OnInterrupted`
            (goto _label))
          (:`OnCancelled`
            (goto _label))))
      (:`OnFailed`
        ; End the ability if there were no blocking hits
        (`self.K2_EndAbility`)))))

(fn `CanCommitAbility`
  (returns (ReturnValue :type Boolean))
  (bind _returnvalue (`self.K2_CheckAbilityCost`))
  (bind _returnvalue_2 (`self.K2_CheckAbilityCooldown`))
  (return (and _returnvalue _returnvalue_2)))

(fn `PitchOverrideCalculation`
  (params (MontageTag :type "GameplayTag Structure (by ref)") (DistanceScale :type "Float (double-precision)") (MaxPitch :type "Float (double-precision)"))
  (returns (ReturnValue :type "Float (double-precision)"))
  (bind _maxpitch (`local.MaxPitch`))
  (bind _asaura_combat_interface (cast `AuraCombatInterface` (`self.GetAvatarActorFromActorInfo`))
    (:`then`
      (return (`KismetMathLibrary.FMin` (* (/ (`KismetMathLibrary.Vector_Distance` (`self.ProjectileTargetLocation`) (`AuraCombatInterface.GetCombatSocketLocation` _asaura_combat_interface (`local.MontageTag`))) (`local.DistanceScale`)) _maxpitch) _maxpitch)))
    (:`CastFailed`
      (return 0.0))))