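; BP_FireBall is a Fire Blast ability actor that flies out and returns to its instigator like a boomerang.
; On the server, StartOutgoingTimeline lerps it from its spawn location to an apex TravelDistance ahead.
; A returning timeline then lerps it toward the instigator's live location.
; It plays hit effects and destroys itself within ExplodeDistance, or is destroyed when the return timeline ends.
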(event `self.StartOutgoingTimeline`
  (bind _returnvalue (`self.GetInstigator`))
  (`/Engine/EditorBlueprintResources/ActorMacros.Switch Has Authority`
    (:`Authority`
      ; Initial location
      (bind _output_get (set `self.InitialLoction` (`self.K2_GetActorLocation`)))
      ; Apex Location
      (set `self.ApexLocation` (+ _output_get (* (`self.GetActorForwardVector`) (`self.TravelDistance`))))
      ; Outgoing Movement
      (bind (_direction _outgoingtrack) (`Timeline|OutgoingTimeline`)
        (:`Update`
          (`self.K2_SetActorLocation` (`KismetMathLibrary.VLerp` (`self.InitialLoction`) (`self.ApexLocation`) _outgoingtrack)))
        (:`Finished`
          ; Returning Movement
          (bind (_direction_2 _returningtrack) (`Timeline|ReturningTimeline`)
            (:`Update`
              (`self.K2_SetActorLocation` (`KismetMathLibrary.VLerp` (`self.ApexLocation`) (`self.K2_GetActorLocation` _returnvalue) _returningtrack))
              ; If close enough, then explode
              (if (< (`self.GetDistanceTo` _returnvalue) (`self.ExplodeDistance`))
                (`self.PlayEffectsOnHit`)
                (`self.K2_DestroyActor`)))
            (:`Finished`
              (`self.K2_DestroyActor`))))))))

(fn `UserConstructionScript`)