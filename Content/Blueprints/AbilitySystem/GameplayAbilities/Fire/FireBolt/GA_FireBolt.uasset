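; GA_FireBolt is a Gameplay Ability that casts a Fire Bolt projectile toward the point under the mouse.
; On valid target data, it stores the hit location, turns the avatar to face it through AuraCombatInterface, and plays the cast montage.
; A montage-driven gameplay event times SpawnProjectile to the arm's full stretch, and the ability ends after a short delay.
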(event `self.K2_ActivateAbility`
  (bind (_asynctaskproxy _datahandle) (`AuraTargetDataUnderMouse.CreateTargetDataUnderMouse`)
    (:`ValidData`
      (set `self.ProjectileTargetLocation` (`.Location` (`GameplayStatics.BreakHitResult` (`AbilitySystemBlueprintLibrary.GetHitResultFromTargetData` _datahandle))))
      ; When this Ability is activated, rotate the character towards the target, play the Fire Bolt montage and when the arm is full stretched emit a Gameplay Event to spawn the projectile
      (bind _asaura_combat_interface (cast `AuraCombatInterface` (`self.GetAvatarActorFromActorInfo`)))
      (`AuraCombatInterface.UpdateFacingTarget` _asaura_combat_interface (`self.ProjectileTargetLocation`))
      (`AbilityTask_PlayMontageAndWait.CreatePlayMontageAndWaitProxy` "None" "/Game/Assets/Characters/Aura/Animations/Abilities/AM_Cast_FireBolt.AM_Cast_FireBolt"
        (:`then`
          (`AbilityTask_WaitGameplayEvent.WaitGameplayEvent` (struct :`TagName` "Event.Montage.FireBolt") null
            (:`EventReceived`
              (`self.SpawnProjectile` (`self.ProjectileTargetLocation`))
              (`KismetSystemLibrary.Delay` 0.5)
              (`self.K2_EndAbility`))))))))