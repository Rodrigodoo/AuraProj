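; Enemy ranged attack gameplay ability that fires a projectile at the avatar's current combat target.
; On activation it turns the avatar toward the target via the combat interface, caches that location and plays a random attack montage.
; The montage's gameplay event tag triggers the projectile spawn toward the cached location.
; The ability ends when the montage completes, is interrupted or cancelled, or when no montage is found.
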(event `self.K2_ActivateAbility`
  (bind _returnvalue (`self.GetAvatarActorFromActorInfo`))
  (bind (_montage _montagetag) (break `TaggedMontage` (`self.TaggedMontage`)))
  ; Update Facing Target to the current Combat Target Actor
  (bind _returnvalue_2 (message `AuraEnemyInterface.GetCombatTarget` _returnvalue))
  (bind _asaura_combat_interface (cast `AuraCombatInterface` _returnvalue))
  (bind _returnvalue_3 (`Actor.K2_GetActorLocation` _returnvalue_2))
  (`AuraCombatInterface.UpdateFacingTarget` _asaura_combat_interface _returnvalue_3)
  (set `self.projectileTarget` _returnvalue_3)
  ; Get a random attack montage from the available montages
  (bind (_randommontage _returnvalue_4) (message `AuraCombatInterface.FindRandomAttackMontage` (`self.GetAvatarActorFromActorInfo`)))
  (if _returnvalue_4
    (set `self.TaggedMontage` _randommontage)
    ; Play the ranged attack montage
    (`AbilityTask_PlayMontageAndWait.CreatePlayMontageAndWaitProxy` "None" _montage 1.0 "None" false
      (:`then`
        (`AbilityTask_WaitGameplayEvent.WaitGameplayEvent` _montagetag null true
          (:`EventReceived`
            ; Spawn the projectile from the socket location of the montage towards the Target location
            (`self.SpawnProjectile` (`self.projectileTarget`) _montagetag))))
      (:`OnCompleted`
        (`self.K2_EndAbility` :!label _label))
      (:`OnInterrupted`
        (goto _label))
      (:`OnCancelled`
        (goto _label)))
    (else
      (`self.K2_EndAbility`))))