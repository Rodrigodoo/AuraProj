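; GA_HitReact is an enemy gameplay ability that plays a hit reaction on its avatar.
; On activation it applies GE_HitReact to the owner, stores the handle, then plays the montage supplied by the avatar's AuraCombatInterface.
; When the montage completes, is interrupted or is cancelled, it removes the effect and ends the ability.
; OnEndAbility also removes the effect by that handle, covering other ways the ability ends.
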(event `self.K2_ActivateAbility`
  ; Apply Hit React Effect
  (bind _returnvalue (`self.BP_ApplyGameplayEffectToOwner` "/Game/Blueprints/AbilitySystem/Enemy/Effects/GE_HitReact.GE_HitReact_C"))
  (set `self.ActiveGEHitReact` _returnvalue)
  ; Play Hit React Montage
  (bind _asaura_combat_interface (cast `AuraCombatInterface` (`self.GetAvatarActorFromActorInfo`)))
  (bind _returnvalue_2 (`AuraCombatInterface.GetHitReactMontage` _asaura_combat_interface))
  (`AbilityTask_PlayMontageAndWait.CreatePlayMontageAndWaitProxy` "None" _returnvalue_2
    (:`OnCompleted`
      _)
    (:`OnInterrupted`
      _)
    (:`OnCancelled`
      _))
  ; Remove Effect and End Ability
  (`self.BP_RemoveGameplayEffectFromOwnerWithHandle` (`self.ActiveGEHitReact`))
  (`self.K2_EndAbility`))

(event `self.K2_OnEndAbility`
  (params (bWasCancelled :type Boolean))
  (`self.BP_RemoveGameplayEffectFromOwnerWithHandle` (`self.ActiveGEHitReact`)))