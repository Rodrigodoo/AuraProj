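; Enemy melee attack ability that turns the avatar toward its combat target and plays a randomly chosen attack montage.
; The montage's tagged gameplay event triggers a small radius check at the matching combat socket, damaging live non-friendly characters.
; On a hit, it executes the MeleeImpact gameplay cue for sound and blood, passing the montage tag, socket location and combat target.
; The ability ends after that event or when the montage finishes.
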(event `self.K2_ActivateAbility`
  (bind _returnvalue (`self.GetAvatarActorFromActorInfo`))
  (bind _returnvalue_2 (`self.GetAvatarActorFromActorInfo`))
  (bind (_montage _montagetag) (break `TaggedMontage` (`self.TaggedMontage`)))
  (set `self.HasHitTarget` false)
  ; Update Facing Target to the current Combat Target Actor
  (bind _returnvalue_3 (message `AuraEnemyInterface.GetCombatTarget` _returnvalue_2))
  (bind _asaura_combat_interface (cast `AuraCombatInterface` _returnvalue_2))
  (`AuraCombatInterface.UpdateFacingTarget` _asaura_combat_interface (`Actor.K2_GetActorLocation` _returnvalue_3))
  ; Get a random attack montage from the available montages
  (bind (_randommontage _returnvalue_4) (message `AuraCombatInterface.FindRandomAttackMontage` (`self.GetAvatarActorFromActorInfo`)))
  (if _returnvalue_4
    (set `self.TaggedMontage` _randommontage)
    ; Play the melee attack montage
    (`AbilityTask_PlayMontageAndWait.CreatePlayMontageAndWaitProxy` "None" _montage 1.0 "None" false
      (:`then`
        ; Get live characters within a radius of the melee weapon tip
        (`AbilityTask_WaitGameplayEvent.WaitGameplayEvent` _montagetag null
          (:`EventReceived`
            (bind _returnvalue_5 (message `AuraCombatInterface.GetCombatSocketLocation` _returnvalue _montagetag))
            (bind _output_get (set `self.CombatSocketLocation` _returnvalue_5))
            (bind _outoverlappingactors (`AuraAbilitySystemLibrary.GetLivePlayerWithinRadius` _returnvalue (`|MakeArray` _returnvalue) 45.0 _output_get))
            (for _array_element _outoverlappingactors
              ; Cause damage to enemies
              (if (`AuraAbilitySystemLibrary.IsNotFriend` (`self.GetAvatarActorFromActorInfo`) _array_element)
                (`AuraAbilitySystemLibrary.ApplyDamageGameplayEffect` (`self.MakeDamageEffectParamsFromClassDefaults` _array_element))
                (set `self.HasHitTarget` true)))
            ; Play Impact Sound and Spawn Blood Effects
            (`self.SpawnSoundAndEffects`)
            (`self.K2_EndAbility`))))
      (:`OnCompleted`
        (`self.K2_EndAbility` :!label _label))
      (:`OnInterrupted`
        (goto _label))
      (:`OnCancelled`
        (goto _label)))
    (else
      (`self.K2_EndAbility`))))

(fn `SpawnSoundAndEffects`
  (bind _returnvalue (`self.GetAvatarActorFromActorInfo`))
  (bind (_taggedmontage_montage _taggedmontage_montagetag) (break `TaggedMontage` (`self.TaggedMontage`)))
  (if (`self.HasHitTarget`)
    ; Execute a Static Gameplay Cue to Spawn the Sound of Impact and the Blood Effect
    (bind _returnvalue_2 (message `AuraEnemyInterface.GetCombatTarget` _returnvalue))
    (`self.K2_ExecuteGameplayCueWithParams` (struct :`TagName` "GameplayCue.MeleeImpact") (`AbilitySystemBlueprintLibrary.MakeGameplayCueParameters` 0.0 0.0 (struct) (struct) (struct) (`BlueprintGameplayTagLibrary.MakeGameplayTagContainerFromTag` _taggedmontage_montagetag) (struct) (`self.CombatSocketLocation`) (0.0 0.0 0.0) null _returnvalue _returnvalue_2))))