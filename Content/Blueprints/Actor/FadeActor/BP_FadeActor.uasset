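; Actor that fades its mesh out and back in, running that cycle on BeginPlay with a short delay between.
; Construction caches the original materials and builds dynamic instances from the fade materials.
; FadeOut swaps these in and plays a timeline driving their Fade parameter, which FadeIn reverses from the end.
; On finish, full Fade restores original materials and Visibility blocking, while zero makes the mesh ignore that channel.
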(event `FadeOut`
  (`self.SetMaterialToDynamicInstances`)
  (bind (_direction _fade) (`Timeline|FadeTimeline` :!label _label)
    (:`Update`
      (for _array_element (`self.DynamicMaterialInstances`)
        (`MaterialInstanceDynamic.SetScalarParameterValue` _array_element "Fade" _fade)))
    (:`Finished`
      (`self.FadeFinished` _fade))))

(event `FadeIn`
  (goto _label :!via `ReverseFromEnd`))

(event `self.ReceiveBeginPlay`
  (`self.FadeOut`)
  (`KismetSystemLibrary.Delay` 1.0)
  (`self.FadeIn`))

(fn `FadeFinished`
  (params (Fade :type "Float (double-precision)"))
  (locals (CollisionResponse :type "ECollisionResponse Enum" :default "ECR_Block"))
  ; If by the end of the timeline our fading is disabled (>=1) then reset the materials to their originals and reisntate the blocking of visibility
  (if (>= Fade 1.0)
    (`self.ResetMaterials`)
    (set `local.CollisionResponse` "ECR_Block")
    (`PrimitiveComponent.SetCollisionResponseToChannel` (`self.Mesh`) "ECC_Visibility" (`local.CollisionResponse`) :!label _label)
    (else
      ; If the actor is faded (<=0) then remove the visibility blocking collision
      (if (<= (`local.Fade`) 0.0)
        (set `local.CollisionResponse` "ECR_Ignore")
        (goto _label)))))

(fn `ResetMaterials`
  (for (_array_element _array_index) (`self.OriginalMaterials`)
    (`PrimitiveComponent.SetMaterial` (`self.Mesh`) _array_index _array_element)))

(fn `SetMaterialToDynamicInstances`
  (for (_array_element _array_index) (`self.DynamicMaterialInstances`)
    (`PrimitiveComponent.SetMaterial` (`self.Mesh`) _array_index _array_element)))

(fn `UserConstructionScript`
  ; Create dynamic material instances for all the materials present in the mesh
  (`KismetArrayLibrary.Array_Clear` (`self.DynamicMaterialInstances`))
  (set `self.OriginalMaterials` (`MeshComponent.GetMaterials` (`self.Mesh`)))
  (for _array_element (`self.FadeMaterialInstances`)
    (bind _returnvalue (`KismetMaterialLibrary.CreateDynamicMaterialInstance` _array_element))
    (`KismetArrayLibrary.Array_AddUnique` (`self.DynamicMaterialInstances`) _returnvalue)))