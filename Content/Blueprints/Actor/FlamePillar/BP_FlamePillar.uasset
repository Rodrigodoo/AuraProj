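; Flame pillar actor whose point light flickers like fire.
; On BeginPlay it makes a dynamic instance of the light's light function material, setting flicker speed, lowest brightness and a random shift so each pillar flickers differently.
; An educational alternative randomly chains two timelines that scale light intensity from a base value, but nothing triggers it, so only the material-driven flicker runs.
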(event `self.ReceiveBeginPlay`
  (`self.InitializeFlickeringLightFunction`))

(event `ChooseTimeline`
  ; Educational - Using timelines to flicker light
  ;; Randomly choose which timeline to use
  (switch `int` (`KismetMathLibrary.RandomIntegerInRange` 0 1)
    (:`Default`
      (`self.StartTimeline2` :!label _label))
    (:`0`
      (`self.StartTimeline1`))
    (:`1`
      (goto _label))))

(event `StartTimeline1`
  ; Educational - Using timelines to flicker light
  ;; Use timelines to flicker the light intensity - When finished use the randomize again
  (bind (_direction _flameintensity) (`Timeline|FlameIntensitiy1` :!via `PlayFromStart`)
    (:`Update`
      (`self.ScaleFlameIntensity` _flameintensity))
    (:`Finished`
      (`self.ChooseTimeline`))))

(event `StartTimeline2`
  ; Educational - Using timelines to flicker light
  ;; Use timelines to flicker the light intensity - When finished use the randomize again
  (bind (_direction _flameintensity) (`Timeline|FlameIntensity2` :!via `PlayFromStart`)
    (:`Update`
      (`self.ScaleFlameIntensity` _flameintensity))
    (:`Finished`
      (`self.ChooseTimeline`))))

(fn `InitializeFlickeringLightFunction`
  ; Set the Point Light's light function and create a random value to make sure each asset flickers differently
  (bind _returnvalue (`KismetMaterialLibrary.CreateDynamicMaterialInstance` (`LightComponent.LightFunctionMaterial` (`self.FireLight`))))
  (`LightComponent.SetLightFunctionMaterial` (`self.FireLight`) _returnvalue)
  (`MaterialInstanceDynamic.SetScalarParameterValue` _returnvalue "RandomnessShift" (`KismetMathLibrary.RandomFloatInRange` -0.5 0.5))
  ; Set flickering speed and lowest brightness
  (`MaterialInstanceDynamic.SetScalarParameterValue` _returnvalue "FlickeringSpeed" 0.3)
  (`MaterialInstanceDynamic.SetScalarParameterValue` _returnvalue "LowestBrightness" 0.6))

(fn `ScaleFlameIntensity`
  (params (FlameIntensityMultiplier :type "Float (double-precision)"))
  (`LightComponent.SetIntensity` (`self.FireLight`) (* FlameIntensityMultiplier (`self.BaseIntensity`))))

(fn `UserConstructionScript`)